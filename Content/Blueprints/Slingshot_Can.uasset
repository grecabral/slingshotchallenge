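; Physics can target for a slingshot game that plays a tin-can sound on impact and reports whether it has been knocked out.
; At start it briefly applies a SixDOF constraint mode to the cylinder, then clears it.
; Tick flags fast movement as flying; only then do hits sound, with ground hits silenced after the first sound via a Gate.
; GetKnockedout checks tilt, height and sideways position against fixed world-space limits.
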(event `self.ReceiveHit`
  (params (MyComp :type "PrimitiveComponent Object Reference") (Other :type "Actor Object Reference") (OtherComp :type "PrimitiveComponent Object Reference") (bSelfMoved :type Boolean) (HitLocation :type "Vector Structure") (HitNormal :type "Vector Structure") (NormalImpulse :type "Vector Structure") (Hit :type "HitResult Structure (by ref)"))
  (if (`self.Flying`)
    (if (`KismetStringLibrary.Contains` (`KismetSystemLibrary.GetDisplayName` Other) "Ground")
      (`/Engine/EditorBlueprintResources/StandardMacros.Gate` false :!label _label
        (:`Exit`
          _)))
    (`GameplayStatics.PlaySound2D` "/Game/Assets/Sounds/240800__ryanconway__hitting-a-tin-can.240800__ryanconway__hitting-a-tin-can" 1.0 1.3)
    (goto _label :!via `Close`)))

(event `self.ReceiveBeginPlay`
  (bind _cylinder (`self.Cylinder`))
  ;[1 1 1] Start Physics settings
  (`PrimitiveComponent.SetConstraintMode` _cylinder "SixDOF")
  (`KismetSystemLibrary.Delay` 2.0)
  (`PrimitiveComponent.SetConstraintMode` _cylinder "None"))

(event `self.ReceiveTick`
  (params (DeltaSeconds :type "Float (single-precision)"))
  (set `self.Flying` (> (`KismetMathLibrary.VSize` (`self.GetVelocity`)) 700.0)))

(fn `Get Knockedout`
  (returns (Knockedout :type Boolean))
  (bind _y (.y (`SceneComponent.K2_GetComponentLocation` (`self.Cylinder`))))
  (return (or (< (.z (`SceneComponent.GetUpVector` (`self.Cylinder`))) 0.5) (< (.z (`SceneComponent.K2_GetComponentLocation` (`self.Cylinder`))) 150.0) (or (< _y 34.0) (> _y 141.0)))))

(fn `UserConstructionScript`)