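; NetworkedCamera is a camera actor that animates between left and right positions and announces when each move ends.
; StartToLeft plays the CameraForLeft timeline for the opening move, then calls StartFinished.
; ToggleLocation plays the ToggleCameraPosition timeline forward for left or reverses it from the end for right, then calls CameraTransitionFinished.
; Both timelines drive X and Y through teleporting SetActorLocation updates, preserving the actor's current Z.
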(event `Start To Left`
  ;[1 1 1] Start transition to left
  (bind (_direction _camerapos) (`Timeline|Camera For Left` :!via `PlayFromStart`)
    (:`Update`
      (`self.K2_SetActorLocation` (`KismetMathLibrary.MakeVector` (.x _camerapos) (.y _camerapos) (.z (`self.K2_GetActorLocation`))) false true))
    (:`Finished`
      (`self.StartFinished`))))

(event `Toggle Location`
  (params (isLeft :type Boolean))
  ;[1 1 1] Camera transition to left and right
  (if isLeft
    (bind (_direction _camera_pos) (`Timeline|Toggle Camera Position` :!via `PlayFromStart` :!label _label)
      (:`Update`
        (`self.K2_SetActorLocation` (`KismetMathLibrary.MakeVector` (.x _camera_pos) (.y _camera_pos) (.z (`self.K2_GetActorLocation`))) false true))
      (:`Finished`
        (`self.CameraTransitionFinished`)))
    (else
      (goto _label :!via `ReverseFromEnd`))))

(fn `UserConstructionScript`)