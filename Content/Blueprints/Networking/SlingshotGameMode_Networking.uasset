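; Server game mode for a two-player networked slingshot can game, running matches from player info exchange through pre-match, rounds and replay.
; Tick starts setup at two players, then advances the round state once both server and client flags report in.
; Events relay holder positions, launches, scores and phase changes through each player state.
; It records per-round scores and cooperation intent, saving match JSON in research mode.
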(event `self.ReceiveBeginPlay`
  (set `self.IsTraveling` false)
  ;[1 1 1] Performance
  (`KismetSystemLibrary.ExecuteConsoleCommand` "r.MaterialQualityLevel 0")
  ;[1 1 1] HTTP Actor
  (`|SpawnActorFromClass` "/Game/Blueprints/Networking/BP_HttpActor.BP_HttpActor_C" (`KismetMathLibrary.MakeTransform` (0.0 0.0 0.0)) "Undefined" "OverrideRootScale"))

(event `self.ReceiveTick`
  (params (DeltaSeconds :type "Float (single-precision)"))
  ;[1 1 1] Checking for logged players to start game logic
  (`|ExecutionSequence`
    (:`then_0`
      (if (== (`KismetArrayLibrary.Array_Length` (`GameStateBase.PlayerArray` (`GameplayStatics.GetGameState`))) 2)
        (`/Engine/EditorBlueprintResources/StandardMacros.DoOnce` false
          (:`Completed`
            (`self.Fixed Begin Play`)))))
    (:`then_1`
      ;[1 1 1] Checking for game state and wait for both clients to update their status
      (switch `/Game/Misc/Enum_RoundStates` (`self.RoundState`)
        (:`NewEnumerator4`
          (if (and (`self.RequestInfo Server`) (`self.RequestInfo Client`))
            (`self.Send Pre-match`)
            (set `self.RequestInfo Server` false)
            (set `self.RequestInfo Client` false)))
        (:`NewEnumerator0`
          (if (and (`self.Pre-Match Server`) (`self.Pre-Match Client`))
            (`self.Send End Pre-Match`)
            (set `self.Pre-Match Server` false)
            (set `self.Pre-Match Client` false)))
        (:`NewEnumerator1`
          (if (and (`self.Turn-End Server`) (`self.Turn-End Client`))
            (`self.Send Turn End`)
            (set `self.Turn-End Server` false)
            (set `self.Turn-End Client` false)))
        (:`NewEnumerator2`
          (if (and (`self.Turn-Ended Server`) (`self.Turn-Ended Client`))
            (`self.Send End-turn event end`)
            (set `self.Turn-Ended Server` false)
            (set `self.Turn-Ended Client` false)))
        (:`NewEnumerator3`
          (if (and (`self.ReplayServer`) (`self.ReplayClient`))
            (`self.Replay Game with same settings`)
            (set `self.ReplayServer` false)
            (set `self.ReplayClient` false)))))))

(event `Update Slingshots Holder Position`
  (params (isServer :type Boolean) (`Relative Position` :type "Vector Structure"))
  ;[1 0 0] Receiving Slingshot's Holder position to update on clients
  (for _array_element (`self.GetPlayerArray`)
    (bind _asslingshot_controller_network (cast `/Game/Blueprints/Networking/SlingshotController_Network` (`self.GetOwner` _array_element)))
    (bind _returnvalue (`Controller.IsLocalController` _asslingshot_controller_network))
    (if (or (and (not _returnvalue) isServer) (and _returnvalue (not isServer)))
      (bind _asslingshot_player_state_networking (cast `/Game/Blueprints/Networking/SLingshotPlayerState_Networking` _array_element))
      (`/Game/Blueprints/Networking/SLingshotPlayerState_Networking.Update Slingshots Holder Position on Client` _asslingshot_player_state_networking `Relative Position`))))

(event `Send Launch information to Clients`
  (params (`Launch Vector` :type "Vector Structure") (isServer :type Boolean))
  ;[1 0 0] Receiving Launch vector from one player to another
  (for _array_element (`self.GetPlayerArray`)
    (bind _asslingshot_controller_network (cast `/Game/Blueprints/Networking/SlingshotController_Network` (`self.GetOwner` _array_element)))
    (bind _returnvalue (`Controller.IsLocalController` _asslingshot_controller_network))
    (if (or (and isServer (not _returnvalue)) (and _returnvalue (not isServer)))
      (bind _asslingshot_player_state_networking (cast `/Game/Blueprints/Networking/SLingshotPlayerState_Networking` _array_element))
      (`/Game/Blueprints/Networking/SLingshotPlayerState_Networking.Receive Launch vector` _asslingshot_player_state_networking `Launch Vector`))))

(event `Fixed Begin Play`
  ;[0 1 0] All clients logged-in, ask for Player information to start the game
  (`self.Set Parameters`)
  (`self.Send Request for Player Data`))

(event `Send Request for Player Data`
  ;[0 1 0] All clients logged-in, ask for Player information to start the game
  (set `self.RoundState` "NewEnumerator4")
  (for _array_element (`self.GetPlayerArray`)
    (bind _asslingshot_player_state_networking (cast `/Game/Blueprints/Networking/SLingshotPlayerState_Networking` _array_element))
    (`/Game/Blueprints/Networking/SLingshotPlayerState_Networking.Receive player info request` _asslingshot_player_state_networking)))

(event `Send Pre-match`
  ;[0 1 0] Starting the game, going for pre-match state
  (set `self.RoundState` "NewEnumerator0")
  (for _array_element (`self.GetPlayerArray`)
    (bind _asslingshot_player_state_networking (cast `/Game/Blueprints/Networking/SLingshotPlayerState_Networking` _array_element))
    (bind (_cooppoints1 _noncooppoints1) (`self.Get Coop And No Coop Points`))
    (`/Game/Blueprints/Networking/SLingshotPlayerState_Networking.Pre-Match` _asslingshot_player_state_networking (`self.Difficulty`) (`self.CansPerRow`) (`self.CanScale`) (`self.CanSize`) (`self.CanPositionsP1`) (`self.CanPositionsP2`) (`self.Round TIme`) (`self.P1 Color`) (`self.P2 Color`) (`self.Number of Rounds`) _cooppoints1 _noncooppoints1)))

(event `Receive Score for Players`
  (params (`P1 Score` :type Integer) (`P2 Score` :type Integer) (`Server Launch` :type Boolean))
  ;[1 0 0] Receiving player scores and relaying to all clients
  (set `self.P1 Score` (+ `P1 Score` (`self.P1 Score`)))
  (set `self.P2 Score` (+ `P2 Score` (`self.P2 Score`)))
  (for _array_element (`self.GetPlayerArray`)
    (bind _asslingshot_player_state_networking (cast `/Game/Blueprints/Networking/SLingshotPlayerState_Networking` _array_element))
    (`/Game/Blueprints/Networking/SLingshotPlayerState_Networking.Receive Scores` _asslingshot_player_state_networking (`self.P1 Score`) (`self.P2 Score`)))
  ;;[0 0 1] Setting variables to record round data
  (set `self.P1 Score on Round` (+ (`self.P1 Score on Round`) `P1 Score`))
  (set `self.P2 Score on Round` (+ `P2 Score` (`self.P2 Score on Round`))))

(event `Send End Pre-Match`
  ;[0 1 0] End of pre match, call round start
  (set `self.RoundState` "NewEnumerator1")
  (for _array_element (`self.GetPlayerArray`)
    (bind _asslingshot_player_state_networking (cast `/Game/Blueprints/Networking/SLingshotPlayerState_Networking` _array_element))
    (`/Game/Blueprints/Networking/SLingshotPlayerState_Networking.Round Start` _asslingshot_player_state_networking (`self.Turn`) false)))

(event `End Pre-Match`
  (params (isServer :type Boolean) (`Player Data` :type "PlayerData Structure"))
  ;[0 1 0] End of pre match, call round start
  (if isServer
    (set `self.Pre-Match Server` true)
    (else
      (set `self.Pre-Match Client` true))))

(event `Receive Player Data`
  (params (`Player Data` :type "PlayerData Structure") (isServer :type Boolean) (`Player Color` :type "LinearColor Structure") (WantsToRecordData :type Boolean))
  ;[1 0 0] Receiving players' data from clients
  (`KismetArrayLibrary.Array_Add` (`self.PlayerData`) `Player Data`)
  (if isServer
    (bind ___ (`self.color!=` (`self.P2 Color`) `Player Color`))
    (if ___
      (set `self.P1 Color` `Player Color`)
      (else
        (set `self.P1 Color` (`self.Default color`))))
    (set `self.RequestInfo Server` true)
    (else
      (bind ____2 (`self.color!=` (`self.P1 Color`) `Player Color`))
      (if ____2
        (set `self.P2 Color` `Player Color`)
        (else
          (set `self.P2 Color` (`self.Default color`))))
      (set `self.RequestInfo Client` true)))
  (if WantsToRecordData
    (bind _gi (`self.Get Game Instance`))
    (set `/Game/Blueprints/SlingshotGameInstance_Networking.usingResearchMode` true _gi)))

(event `Turn Has Ended`
  (params (isServer :type Boolean) (IgnoreIntent :type Boolean) (LeftIntent :type Boolean))
  (bind _returnvalue (not LeftIntent))
  (bind _altcanspawn (`self.altCanSpawn`))
  ;[0 1 0] End of turn
  (if isServer
    (set `self.Turn-End Server` true)
    (if IgnoreIntent
      _
      (elif _altcanspawn
        (set `self.P1 Launch Left Intent` LeftIntent)
        (else
          (set `self.P1 Launch Left Intent` _returnvalue))))
    (else
      (set `self.Turn-End Client` true)
      (if IgnoreIntent
        _
        (elif _altcanspawn
          (set `self.P2 Launch Left Intent` LeftIntent)
          (else
            (set `self.P2 Launch Left Intent` _returnvalue)))))))

(event `Send Turn End`
  ;[0 1 0] End of turn
  (set `self.RoundState` "NewEnumerator2")
  (for _array_element (`self.GetPlayerArray`)
    (bind _asslingshot_player_state_networking (cast `/Game/Blueprints/Networking/SLingshotPlayerState_Networking` _array_element))
    (`/Game/Blueprints/Networking/SLingshotPlayerState_Networking.Receive End turn` _asslingshot_player_state_networking (`self.Turn`))))

(event `self.K2_OnLogout`
  (params (ExitingController :type "Controller Object Reference"))
  ;[1 0 1] Client disconnected
  (if (and (not (`Controller.IsLocalController` ExitingController)) (not (`self.IsTraveling`)))
    (bind _returnvalue (`|CreateWidget` "/Game/Huds/W_ErrorMessages.W_ErrorMessages_C"))
    (`UserWidget.AddToViewport` _returnvalue 0)
    (`TextBlock.SetText` (`/Game/Huds/W_ErrorMessages.ErrorMessage` _returnvalue) "Player 2 saiu")))

(event `End-Turn event has ended`
  (params (isServer :type Boolean))
  ;[0 1 0] End-turn event has ended, call round start on all clients or end the game
  (if isServer
    (set `self.Turn-Ended Server` true)
    (else
      (set `self.Turn-Ended Client` true))))

(event `Send End-turn event end`
  ;[0 1 0] End-turn event has ended, call round start on all clients or end the game
  (if (== (mod (`self.Turn`) 2) 0)
    (`self.Save Round Data` (`self.P1 Score on Round`) (`self.P2 Score on Round`))
    (set `self.P1 Score on Round` 0)
    (set `self.P2 Score on Round` 0))
  (if (!= (/ (`self.Turn`) 2) (`self.Number of Rounds`))
    (set `self.RoundState` "NewEnumerator1")
    (`/Engine/EditorBlueprintResources/StandardMacros.IncrementInt` (`self.Turn`)
      (:`  `
        (if (== (mod (`self.Turn`) 2) 1)
          (set `self.altCanSpawn` (not (`self.altCanSpawn`))))
        (for _array_element (`self.GetPlayerArray`)
          (bind _asslingshot_player_state_networking (cast `/Game/Blueprints/Networking/SLingshotPlayerState_Networking` _array_element))
          (`/Game/Blueprints/Networking/SLingshotPlayerState_Networking.Round Start` _asslingshot_player_state_networking (`self.Turn`) (`self.altCanSpawn`)))))
    (else
      (`self.Save Match Data`)
      (set `self.RoundState` "NewEnumerator3")
      (for _array_element_2 (`self.GetPlayerArray`)
        (bind _asslingshot_player_state_networking_2 (cast `/Game/Blueprints/Networking/SLingshotPlayerState_Networking` _array_element_2))
        (`/Game/Blueprints/Networking/SLingshotPlayerState_Networking.Receive End Game` _asslingshot_player_state_networking_2)))))

(event `Replay Game with same settings`
  ;[0 1 0] Replay Event
  (bind _asslingshot_game_instance_networking (cast `/Game/Blueprints/SlingshotGameInstance_Networking` (`GameplayStatics.GetGameInstance`)))
  (if (`/Game/Blueprints/SlingshotGameInstance_Networking.usingResearchMode` _asslingshot_game_instance_networking)
    (for _array_element (`self.GetPlayerArray`)
      (bind _asslingshot_player_state_networking (cast `/Game/Blueprints/Networking/SLingshotPlayerState_Networking` _array_element))
      (`/Game/Blueprints/Networking/SLingshotPlayerState_Networking.Receive message from play again` _asslingshot_player_state_networking))
    (else
      (`KismetSystemLibrary.ExecuteConsoleCommand` "ServerTravel Suburb_MP" :!label _label))))

(event `Receive Replay intent`
  (params (isServer :type Boolean))
  ;[0 1 0] Replay Event
  (if isServer
    (set `self.ReplayServer` true)
    (else
      (set `self.ReplayClient` true))))

(event `Reopen level`
  ;[0 1 0] Replay Event
  (set `self.IsTraveling` true)
  (goto _label))

(event `Save Round Data`
  (params (`Player 1Score` :type Integer) (`Player 2Score` :type Integer))
  ;[0 0.002356 1] Saving Round Data
  (`KismetArrayLibrary.Array_Add` (`self.RoundsData`) (make `RoundData` (/ (`self.Turn`) 2) `Player 1Score` `Player 2Score` (select `bool` (`self.P1 Launch Left Intent`) :`false` 1 :`true` 0) (select `bool` (`self.P2 Launch Left Intent`) :`false` 1 :`true` 0))))

(event `Save Match Data`
  ;[0 0 1] Save match Data
  (bind _gi (`self.Get Game Instance`))
  (if (`/Game/Blueprints/SlingshotGameInstance_Networking.usingResearchMode` _gi)
    (bind (_cooppoints1 _noncooppoints1) (`self.Get Coop And No Coop Points`))
    (bind _output_get (set `self.MatchData` (make `MatchData` (`self.PlayerData`) (`self.Number of Rounds`) _cooppoints1 _noncooppoints1 (`KismetMathLibrary.Conv_ByteToInt` (`self.Difficulty`)) 5 (`self.RoundsData`) 1)))
    (`SaveandLoadFiles.saveJsonToFile` _output_get)))

(fn `color!=`
  (params (Color1 :type "LinearColor Structure") (Color2 :type "LinearColor Structure"))
  (returns (`!=` :type Boolean))
  (bind (_r _g _b _a) (`KismetMathLibrary.BreakColor` Color1))
  (bind (_r_2 _g_2 _b_2 _a_2) (`KismetMathLibrary.BreakColor` Color2))
  (return (or (!= _r _r_2) (!= _g _g_2) (!= _b _b_2) (!= _a _a_2))))

(fn `Get Coop And No Coop Points`
  (returns (CoopPoints1 :type Integer) (NonCoopPoints1 :type Integer))
  (locals (CoopPoints :type Integer) (NonCoopPoints :type Integer))
  (for _array_element (`self.CanPositionsP1`)
    (switch `/Game/Misc/Enum_CanValues` _array_element
      (:`NewEnumerator0`
        (`/Engine/EditorBlueprintResources/StandardMacros.IncrementInt` (`local.NonCoopPoints`)))
      (:`NewEnumerator2`
        (`/Engine/EditorBlueprintResources/StandardMacros.IncrementInt` (`local.CoopPoints`)))))
  (for _array_element_2 (`self.CanPositionsP2`)
    (switch `/Game/Misc/Enum_CanValues` _array_element_2
      (:`NewEnumerator0`
        (`/Engine/EditorBlueprintResources/StandardMacros.IncrementInt` (`local.NonCoopPoints`)))
      (:`NewEnumerator2`
        (`/Engine/EditorBlueprintResources/StandardMacros.IncrementInt` (`local.CoopPoints`)))))
  (return (`local.CoopPoints`) (`local.NonCoopPoints`)))

(fn `Set Parameters`
  (bind _asslingshot_game_instance_networking (cast `/Game/Blueprints/SlingshotGameInstance_Networking` (`GameplayStatics.GetGameInstance`))
    (:`then`
      (bind (_players _number_of_rounds _coop_points _no_coop_points _difficulty) (break `MatchData` (`/Game/Blueprints/SlingshotGameInstance_Networking.MatchData` _asslingshot_game_instance_networking)))
      (set `self.Number of Rounds` _number_of_rounds)
      (set `self.CanPositionsP1` (`/Game/Blueprints/SlingshotGameInstance_Networking.CanPositionsP1` _asslingshot_game_instance_networking))
      (set `self.CanPositionsP2` (`/Game/Blueprints/SlingshotGameInstance_Networking.CanPositionsP2` _asslingshot_game_instance_networking))
      (switch `int` _difficulty
        (:`Default`
          (set `self.Difficulty` "NewEnumerator0" :!label _label))
        (:`0`
          (goto _label))
        (:`1`
          (set `self.Difficulty` "NewEnumerator1"))
        (:`2`
          (set `self.Difficulty` "NewEnumerator2"))))
    (:`CastFailed`
      _))
  (return))

(fn `UserConstructionScript`)