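; Networked touch controller for a turn-based slingshot, accepting input only on the local player's turn (odd turns server, even client).
; Pressing the slingshot opens a gate; touch moves then trace a second object type to position the Holder, clamped in X/Z and mirrored by world side.
; Release launches attached projectiles along the Holder-to-AimPosition vector with server update, then resets the Holder.
; Holder positions are forwarded to the networking GameInstance.
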(event `Set Slingshot`
  (params (Slingshot :type "/Game/Blueprints/Networking/NetworkedSlingshot Object Reference"))
  ;[1 1 1] Getting Slingshot Reference
  (set `self.Slingshot` Slingshot))

(event `InputTouch`
  (params (Location :type "Vector Structure") (FingerIndex :type "ETouchIndex Enum"))
  (bind _slingshot (`self.Slingshot`))
  (bind _slingshot_2 (`self.Slingshot`))
  (bind (_hitresult _returnvalue) (`self.GetHitResultUnderFingerForObjects` "Touch1" (`|MakeArray` "ObjectTypeQuery8" :!type "EObjectTypeQuery Enum")))
  (bind (_x _y) (`KismetMathLibrary.BreakVector2D` (`self.ClampBounds`)))
  (bind _x_2 (`KismetMathLibrary.BreakVector2D` (`self.ClampBounds`)))
  (bind _returnvalue_2 (`KismetMathLibrary.MakeVector` (`self.SlingX`) (`self.SlingY`) (`self.SlingZ`)))
  (bind _holder (`/Game/Blueprints/Networking/NetworkedSlingshot.Holder` _slingshot_2))
  (bind _x_3 (.x (`self.K2_GetActorLocation` _slingshot_2)))
  (bind _returnvalue_3 (* _x_2 -1.0))
  (bind _returnvalue_4 (< _x_3 0.0))
  (bind _z (.z (.location (`SceneComponent.GetRelativeTransform` (`/Game/Blueprints/Networking/NetworkedSlingshot.Aim` _slingshot_2)))))
  (bind _x_4 (.x (- (`SceneComponent.K2_GetComponentLocation` (`/Game/Blueprints/Networking/NetworkedSlingshot.AimPosition` _slingshot)) (`SceneComponent.K2_GetComponentLocation` (`/Game/Blueprints/Networking/NetworkedSlingshot.Holder` _slingshot)))))
  (bind _z_2 (.z (- (`SceneComponent.K2_GetComponentLocation` (`/Game/Blueprints/Networking/NetworkedSlingshot.AimPosition` _slingshot)) (`SceneComponent.K2_GetComponentLocation` (`/Game/Blueprints/Networking/NetworkedSlingshot.Holder` _slingshot)))))
  (bind _y_2 (.y (.location (`SceneComponent.GetRelativeTransform` _holder))))
  (bind _returnvalue_5 (`KismetMathLibrary.MakeVector` _x_4 _z_2 _z_2))
  (bind _returnvalue_6 (`KismetMathLibrary.MakeVector` 0.0 _y_2 _z))
  (bind _returnvalue_7 (not (< _x_4 0.0)))
  (bind _returnvalue_8 (- (.z (`.Location` (`GameplayStatics.BreakHitResult` _hitresult))) (+ _z (.z (`self.K2_GetActorLocation` _slingshot_2)))))
  (bind _returnvalue_9 (- (`KismetMathLibrary.Abs` (.x (`.Location` (`GameplayStatics.BreakHitResult` _hitresult)))) (+ (.x (.location (`SceneComponent.GetRelativeTransform` (`/Game/Blueprints/Networking/NetworkedSlingshot.Aim` _slingshot_2)))) (`KismetMathLibrary.Abs` _x_3))))
  (bind _returnvalue_10 (* _returnvalue_9 -1.0))
  (bind _returnvalue_11 (< _returnvalue_10 0.0))
  ;[1 1 1] Setting Slingshot's holder position on Touch movements
  (:`Pressed`
    (`self.IsMyTurn?`)
    (if (== (`.HitActor` (`GameplayStatics.BreakHitResult` (`self.GetHitResultUnderFingerForObjects` "Touch1" (`|MakeArray` "ObjectTypeQuery7" :!type "EObjectTypeQuery Enum")))) (`self.Slingshot`))
      (set `self.isPressedOnSlingshot` true)
      (goto _label :!via `Open`)))
  (:`Released`
    (`self.IsMyTurn?`)
    (`|ExecutionSequence`
      (:`then_0`
        ;[1 1 1] On release
        (if (`self.isPressedOnSlingshot`)
          (for _array_element (`self.GetAttachedActors` _slingshot)
            (bind _asnetworked_slingshot_projectile (cast `/Game/Blueprints/Networking/NetworkedSlingshot_Projectile` _array_element))
            (if (not (`self.LaunchedProjectile`))
              (`/Game/Blueprints/Networking/NetworkedSlingshot_Projectile.LaunchMe` _asnetworked_slingshot_projectile _returnvalue_5 (`KismetMathLibrary.VSize` _returnvalue_5) true _returnvalue_7)
              (set `self.LaunchedProjectile` true)
              (`self.Launch Dispatcher` _returnvalue_7)))))
      (:`then_1`
        (`SceneComponent.K2_SetRelativeLocation` _holder _returnvalue_6 false false)
        (bind _game_instance (`self.Get Game Instance`)
          (:`then`
            (`/Game/Blueprints/SlingshotGameInstance_Networking.Update Slingshots Holder Position` _game_instance _returnvalue_6))))
      (:`then_2`
        (set `self.isPressedOnSlingshot` false)
        (goto _label :!via `Close`))))
  (:`Moved`
    (`self.IsMyTurn?`)
    (`/Engine/EditorBlueprintResources/StandardMacros.Gate` true :!label _label
      (:`Exit`
        (if (not (`self.LaunchedProjectile`))
          (set `self.SlingY` _y_2)
          (`|ExecutionSequence`
            (:`then_0`
              ;;[1 1 1] Clamping X and Z
              ;;;[1 1 1] Clamping X
              (if (> (`KismetMathLibrary.Abs` _returnvalue_9) (`KismetMathLibrary.BreakVector2D` (`self.ClampBounds`)))
                (if _returnvalue_4
                  (if _returnvalue_11
                    (set `self.SlingX` _x_2)
                    (else
                      (set `self.SlingX` _returnvalue_3)))
                  (elif _returnvalue_11
                    (set `self.SlingX` _returnvalue_3)
                    (else
                      (set `self.SlingX` _x_2))))
                (elif _returnvalue_4
                  (set `self.SlingX` _returnvalue_9)
                  (else
                    (set `self.SlingX` _returnvalue_10)))))
            (:`then_1`
              ;;;[1 1 1] Clamping Z
              (if (> (`KismetMathLibrary.Abs` _returnvalue_8) (`.Y` (`KismetMathLibrary.BreakVector2D` (`self.ClampBounds`))))
                (if (< _returnvalue_8 0.0)
                  (set `self.SlingZ` (+ (* _y -1.0) _z))
                  (else
                    (set `self.SlingZ` (+ _y _z))))
                (else
                  (set `self.SlingZ` (+ _z _returnvalue_8)))))
            (:`then_2`
              (if _returnvalue
                (`SceneComponent.K2_SetRelativeLocation` _holder _returnvalue_2 false false)
                (bind _game_instance_2 (`self.Get Game Instance`)
                  (:`then`
                    (`/Game/Blueprints/SlingshotGameInstance_Networking.Update Slingshots Holder Position` _game_instance_2 _returnvalue_2)))))))))))

(fn `UserConstructionScript`)