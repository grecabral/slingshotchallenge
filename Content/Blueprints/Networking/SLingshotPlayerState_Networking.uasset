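; Player state that relays network messages for a two-player, turn-based slingshot can-shooting match.
; Send events cast to the networking GameMode to report pre-match completion, holder position, launch vector, turn ends, scores, player data and replay intent.
; Receive events forward match setup, round and turn changes, opponent input, scores, game end and requests to the networking GameInstance through a cast helper.
; It holds no match logic itself.
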(event `self.ReceiveBeginPlay`)

(event `Pre-Match`
  (params (Difficulty :type "/Game/Misc/Enum_Difficulty Enum") (`Cans Per Row` :type Integer) (`Can Scale Bias` :type "Vector Structure") (`Can Size` :type "Vector2D Structure") (`Can Positions P1` :type "Array of /Game/Misc/Enum_CanValues Enum (by ref)") (`Can Positions P2` :type "Array of /Game/Misc/Enum_CanValues Enum (by ref)") (`Round Time` :type "Float (double-precision)") (`P1 Color` :type "LinearColor Structure") (`P2 Color` :type "LinearColor Structure") (NOfRounds :type Integer) (CoopPoints :type Integer) (NoCoopPoints :type Integer))
  ;[1 1 1] Recieve from Server
  ;;[1 1 1] Pre-Match
  (bind _game_instance (`self.Get Slingshot Game Instance`)
    (:`then`
      (`/Game/Blueprints/SlingshotGameInstance_Networking.Pre-Match` _game_instance Difficulty `Cans Per Row` `Can Scale Bias` `Can Size` `Can Positions P1` `Can Positions P2` `Round Time` `P1 Color` `P2 Color` NOfRounds CoopPoints NoCoopPoints))))

(event `Pre-Match-Ended`
  (params (isServer :type Boolean) (`Player Data` :type "PlayerData Structure"))
  ;[1 1 1] Send to server
  ;;[1 1 1] End of pre-match
  (bind _asslingshot_game_mode_networking (cast `/Game/Blueprints/Networking/SlingshotGameMode_Networking` (`GameplayStatics.GetGameMode`)))
  (`/Game/Blueprints/Networking/SlingshotGameMode_Networking.End Pre-Match` _asslingshot_game_mode_networking isServer `Player Data`))

(event `Send Holder Position to Server`
  (params (isServer :type Boolean) (`Relative Position` :type "Vector Structure"))
  ;[1 1 1] Send to server
  ;;[1 1 1] Sending Slingshot's holder position to server
  (bind _asslingshot_game_mode_networking (cast `/Game/Blueprints/Networking/SlingshotGameMode_Networking` (`GameplayStatics.GetGameMode`)))
  (`/Game/Blueprints/Networking/SlingshotGameMode_Networking.Update Slingshots Holder Position` _asslingshot_game_mode_networking isServer `Relative Position`))

(event `Round Start`
  (params (Turn :type Integer) (AltCanSpawn :type Boolean))
  ;[1 1 1] Recieve from Server
  ;;[1 1 1] Round Start
  (bind _game_instance (`self.Get Slingshot Game Instance`)
    (:`then`
      (`/Game/Blueprints/SlingshotGameInstance_Networking.Round Start` _game_instance Turn AltCanSpawn))))

(event `Send Launch Vector to Server`
  (params (`Launch Vector` :type "Vector Structure") (isServer :type Boolean))
  ;[1 1 1] Send to server
  ;;[1 1 1] Sending ball launch vector to server
  (bind _asslingshot_game_mode_networking (cast `/Game/Blueprints/Networking/SlingshotGameMode_Networking` (`GameplayStatics.GetGameMode`)))
  (`/Game/Blueprints/Networking/SlingshotGameMode_Networking.Send Launch information to Clients` _asslingshot_game_mode_networking `Launch Vector` isServer))

(event `Update Slingshots Holder Position on Client`
  (params (`Relative Position` :type "Vector Structure"))
  ;[1 1 1] Recieve from Server
  ;;[1 1 1] Receive Slingshot's Holder Position
  (bind _game_instance (`self.Get Slingshot Game Instance`)
    (:`then`
      (`/Game/Blueprints/SlingshotGameInstance_Networking.Receive Slingshots Holder Position` _game_instance `Relative Position`))))

(event `Receive Launch vector`
  (params (`Launch Vector` :type "Vector Structure"))
  ;[1 1 1] Recieve from Server
  ;;[1 1 1] Receive Launch Vector from server
  (bind _game_instance (`self.Get Slingshot Game Instance`)
    (:`then`
      (`/Game/Blueprints/SlingshotGameInstance_Networking.Receive Launch information from server` _game_instance `Launch Vector`))))

(event `Send End Turn`
  (params (IsServer :type Boolean) (IgnoreIntent :type Boolean) (LeftIntent :type Boolean))
  ;[1 1 1] Send to server
  ;;[1 1 1] Send information that the turn has ended
  (bind _asslingshot_game_mode_networking (cast `/Game/Blueprints/Networking/SlingshotGameMode_Networking` (`GameplayStatics.GetGameMode`)))
  (`/Game/Blueprints/Networking/SlingshotGameMode_Networking.Turn Has Ended` _asslingshot_game_mode_networking IsServer IgnoreIntent LeftIntent))

(event `Receive End turn`
  (params (Turn :type Integer))
  ;[1 1 1] Recieve from Server
  ;;[1 1 1] Receive order to end turn
  (bind _game_instance (`self.Get Slingshot Game Instance`)
    (:`then`
      (`/Game/Blueprints/SlingshotGameInstance_Networking.End-Turn` _game_instance Turn))))

(event `Send End-Turn has ended`
  (params (IsServer :type Boolean))
  ;[1 1 1] Send to server
  ;;[1 1 1] Send info that the End-turn event has ended
  (bind _asslingshot_game_mode_networking (cast `/Game/Blueprints/Networking/SlingshotGameMode_Networking` (`GameplayStatics.GetGameMode`)))
  (`/Game/Blueprints/Networking/SlingshotGameMode_Networking.End-Turn event has ended` _asslingshot_game_mode_networking IsServer))

(event `Receive Scores`
  (params (`P1 Score` :type Integer) (`P2 Score` :type Integer))
  ;[1 1 1] Recieve from Server
  ;;[1 1 1] Receiving players scores
  (bind _game_instance (`self.Get Slingshot Game Instance`)
    (:`then`
      (`/Game/Blueprints/SlingshotGameInstance_Networking.Receive players score` _game_instance `P1 Score` `P2 Score`))))

(event `Send Score to Server`
  (params (`P1 Points` :type Integer) (`P2 Points` :type Integer) (`Server Launch` :type Boolean))
  ;[1 1 1] Send to server
  ;;[1 1 1] Sending Score to Server
  (bind _asslingshot_game_mode_networking (cast `/Game/Blueprints/Networking/SlingshotGameMode_Networking` (`GameplayStatics.GetGameMode`)))
  (`/Game/Blueprints/Networking/SlingshotGameMode_Networking.Receive Score for Players` _asslingshot_game_mode_networking `P1 Points` `P2 Points` `Server Launch`))

(event `Receive End Game`
  ;[1 1 1] Recieve from Server
  ;;[1 1 1] Receive End Game
  (bind _game_instance (`self.Get Slingshot Game Instance`)
    (:`then`
      (`/Game/Blueprints/SlingshotGameInstance_Networking.End Game` _game_instance))))

(event `Send Player Data to server`
  (params (`Player Data` :type "PlayerData Structure") (isServer :type Boolean) (`Player Color` :type "LinearColor Structure") (wantsToRecordData :type Boolean))
  ;[1 1 1] Send to server
  ;;[1 1 1] Sending Player Data
  (bind _asslingshot_game_mode_networking (cast `/Game/Blueprints/Networking/SlingshotGameMode_Networking` (`GameplayStatics.GetGameMode`)))
  (`/Game/Blueprints/Networking/SlingshotGameMode_Networking.Receive Player Data` _asslingshot_game_mode_networking `Player Data` isServer `Player Color` wantsToRecordData))

(event `Receive player info request`
  ;[1 1 1] Recieve from Server
  ;;[1 1 1] Receive server request for player information
  (bind _game_instance (`self.Get Slingshot Game Instance`)
    (:`then`
      (`/Game/Blueprints/SlingshotGameInstance_Networking.Send Player Data to server` _game_instance))))

(event `Receive message from play again`
  ;[1 1 1] Recieve from Server
  ;;[1 1 1] Receiving message from play again to call dispatcher
  (bind _game_instance (`self.Get Slingshot Game Instance`)
    (:`then`
      (`/Game/Blueprints/SlingshotGameInstance_Networking.PlayAgainDispatcher` _game_instance))))

(event `Send replay intent to server`
  (params (isServer :type Boolean))
  ;[1 1 1] Send to server
  ;;[1 1 1] Receiving replay intent from clients and sending to server
  (bind _asslingshot_game_mode_networking (cast `/Game/Blueprints/Networking/SlingshotGameMode_Networking` (`GameplayStatics.GetGameMode`)))
  (`/Game/Blueprints/Networking/SlingshotGameMode_Networking.Receive Replay intent` _asslingshot_game_mode_networking isServer))

(fn `UserConstructionScript`)