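; BP_HttpActor is a networking actor that periodically checks for saved data and sends it through an HTTP call.
; A looping two-second timer loads the data as a string, guarded by an IsOpen flag, and calls HttpCall when data exists and IsDone is true.
; It toggles the SendingFiles widget and, when the game mode is MainMenuGameMode, shows or hides the menu's data notification through its alpha.
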(event `self.ReceiveBeginPlay`
  (`self.LoadWidget`)
  (`KismetSystemLibrary.K2_SetTimerDelegate` (delegate `Check For Data`) 2.0 true))

(event `Check For Data`
  (if (`self.isOpen`)
    (set `self.isOpen` false)
    (if (not (`Widget.IsVisible` (`self.SendingFiles`)))
      (`Widget.SetVisibility` (`self.SendingFiles`) "Visible"))
    (bind (_isempty _data) (`self.Get Data Files`))
    (if (not _isempty)
      (`self.Show Notification` 1.0
        (:`On Main Menu`
          _)
        (:`Not on Main Menu`
          _))
      (if (`self.isDone`)
        (`self.HttpCall` _data))
      (else
        (`Widget.SetVisibility` (`self.SendingFiles`) "Hidden")
        (`self.Show Notification` 0.0
          (:`On Main Menu`
            _)
          (:`Not on Main Menu`
            _))))
    (set `self.isOpen` true)))

(fn `Get Data Files`
  (returns (isEmpty :type Boolean) (Data :type "Array of FileContent Structure"))
  (bind _returnvalue (`SaveandLoadFiles.LoadDataToString`))
  (return (== (`KismetArrayLibrary.Array_Length` _returnvalue) 0) _returnvalue))

(fn `UserConstructionScript`)