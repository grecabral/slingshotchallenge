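; A can target for a networked slingshot game that can be tinted with a player color and report whether it has been knocked out.
; It holds its cylinder in SixDOF constraint mode briefly at start, then releases it to physics.
; Every tick it passes its transform to UpdatePhysics, which teleports non-server instances to it as a correction.
; GetKnockedout flags the can when it tips over, drops too low or leaves its Y bounds.
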(event `self.ReceiveBeginPlay`
  (bind _cylinder (`self.Cylinder`))
  ;[1 1 1] Start Physics settings
  (`PrimitiveComponent.SetConstraintMode` _cylinder "SixDOF")
  (`KismetSystemLibrary.Delay` 2.0)
  (`PrimitiveComponent.SetConstraintMode` _cylinder "None"))

(event `Change Material`
  (params (Color :type "LinearColor Structure"))
  ;[1 1 1] Changing Color
  (`MeshComponent.SetVectorParameterValueOnMaterials` (`self.Cylinder`) "PlayerColor" (`KismetMathLibrary.Conv_LinearColorToVector` Color)))

(event `self.ReceiveTick`
  (params (DeltaSeconds :type "Float (single-precision)"))
  ;[1 1 1] Update replicated cans physics
  (`self.Update Physics` (`self.GetTransform`)))

(event `Update Physics`
  (params (NewTransform :type "Transform Structure (by ref)"))
  ;[1 1 1] Receive physics corrections
  (if (not (`KismetSystemLibrary.IsServer`))
    (`self.K2_SetActorTransform` NewTransform false true)))

(fn `Get knockedout`
  (returns (Knockedout :type Boolean))
  (bind _y (.y (`SceneComponent.K2_GetComponentLocation` (`self.Cylinder`))))
  (return (or (< (.z (`SceneComponent.GetUpVector` (`self.Cylinder`))) 0.5) (< (.z (`SceneComponent.K2_GetComponentLocation` (`self.Cylinder`))) 150.0) (or (< _y 34.0) (> _y 141.0)))))

(fn `UserConstructionScript`)