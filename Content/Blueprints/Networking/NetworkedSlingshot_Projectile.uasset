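; Projectile for the networked slingshot: it attaches to the slingshot holder on spawn, then launches through projectile movement and pushes what it hits.
; Launch clamps direction and branches on difficulty: Easy snaps to preset vectors, Medium does so only within set bounds, Hard follows the aim.
; Local launches send the direction to the server via the game instance.
; Easy and assisted Medium shots fire a radial impulse on overlap, and hits shove physics bodies.
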(event `self.ReceiveBeginPlay`
  ;[1 1 1] Preparation for proper placement
  (bind _outactors (`GameplayStatics.GetAllActorsOfClass` "/Game/Blueprints/Networking/NetworkedSlingshot.NetworkedSlingshot_C"))
  (set `self.Slingshot` (`KismetArrayLibrary.Array_Get` _outactors))
  (`self.Attach to slingshot`))

(event `Attach to slingshot`
  (bind _holder (`/Game/Blueprints/Networking/NetworkedSlingshot.Holder` (`self.Slingshot`)))
  ;[1 1 1] Setting position based on slingshot holder and attaching myself into it
  (`self.K2_SetActorLocation` (+ (`SceneComponent.K2_GetComponentLocation` _holder) (0.0 5.0 0.0)) false true)
  (`self.K2_AttachToComponent` _holder "None" "KeepWorld" "KeepWorld" "KeepWorld" false))

(event `LaunchMe`
  (params (Direction :type "Vector Structure") (Speed :type "Float (double-precision)") (SendServerUpdate :type Boolean) (LeftIntent :type Boolean))
  (bind _projectilemovement (`self.ProjectileMovement`))
  (bind _projectilemovement_2 (`self.ProjectileMovement`))
  (bind _returnvalue (`KismetMathLibrary.MakeVector` (.x Direction) (`KismetMathLibrary.FClamp` (.y Direction) 0.0 20.0) (`KismetMathLibrary.FClamp` (.z Direction) 0.0 20.0)))
  (bind _returnvalue_2 (`KismetMathLibrary.Abs` (.y _returnvalue)))
  ;[1 1 1] Launch me
  (`|ExecutionSequence`
    (:`then_0`
      (switch `/Game/Misc/Enum_Difficulty` (`self.Difficulty`)
        (:`NewEnumerator0`
          ;;[1 1 1] Easy Logic
          (if (> (.x _returnvalue) 0.0) :!label _label
            (set `MovementComponent.Velocity` (* (`self.Power`) (`KismetArrayLibrary.Array_Get` (`self.EasyLaunchVectors`))) _projectilemovement)
            (`ActorComponent.SetActive` _projectilemovement true false)
            (else
              (set `MovementComponent.Velocity` (* (`KismetArrayLibrary.Array_Get` (`self.EasyLaunchVectors`) 1) (`self.Power`)) _projectilemovement)
              (`ActorComponent.SetActive` _projectilemovement true false))))
        (:`NewEnumerator1`
          ;;[1 1 1] Medium Logic
          (if (and (and (<= (`KismetMathLibrary.Abs` (.x _returnvalue)) (`KismetMathLibrary.BreakVector2D` (`self.MediumBounds`))) (<= _returnvalue_2 (`.Y` (`KismetMathLibrary.BreakVector2D` (`self.MediumBounds`))))) (> _returnvalue_2 (`.Y` (`KismetMathLibrary.BreakVector2D` (`self.MediumGap`)))))
            (set `self.UseForce` true)
            (goto _label)
            (else
              ;;[1 1 1] Hard Logic
              (set `MovementComponent.Velocity` (* _returnvalue (`self.Power`)) _projectilemovement_2 :!label _label_2)
              (`ActorComponent.SetActive` _projectilemovement_2 true false))))
        (:`NewEnumerator2`
          (goto _label_2))))
    (:`then_1`
      ;;[1 1 1] Send Launch information to server
      (if SendServerUpdate
        (bind _asslingshot_game_instance_networking (cast `/Game/Blueprints/SlingshotGameInstance_Networking` (`GameplayStatics.GetGameInstance`)))
        (`/Game/Blueprints/SlingshotGameInstance_Networking.Send Launch Information` _asslingshot_game_instance_networking _returnvalue)
        (`self.Ball Launched` LeftIntent)))))

(event `self.ReceiveActorBeginOverlap`
  (params (OtherActor :type "Actor Object Reference"))
  (bind _radialforce (`self.RadialForce`))
  ;[1 1 1] Launch me
  ;;[1 1 1] On hit Effects
  (switch `/Game/Misc/Enum_Difficulty` (`self.Difficulty`)
    (:`NewEnumerator0`
      (`ActorComponent.Activate` _radialforce false :!label _label_3)
      (`RadialForceComponent.FireImpulse` _radialforce))
    (:`NewEnumerator1`
      (if (`self.UseForce`)
        (goto _label_3)))))

(event `self.ReceiveHit`
  (params (MyComp :type "PrimitiveComponent Object Reference") (Other :type "Actor Object Reference") (OtherComp :type "PrimitiveComponent Object Reference") (bSelfMoved :type Boolean) (HitLocation :type "Vector Structure") (HitNormal :type "Vector Structure") (NormalImpulse :type "Vector Structure") (Hit :type "HitResult Structure (by ref)"))
  ;[1 1 1] Launch me
  ;;[1 1 1] On hit Effects
  ;;;[1 1 1] Impact
  (if (`SceneComponent.IsSimulatingPhysics` OtherComp "None")
    (`PrimitiveComponent.AddImpulseAtLocation` OtherComp (* (`self.GetVelocity`) 10.0) HitNormal "None")))

(fn `UserConstructionScript`)