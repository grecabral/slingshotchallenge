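; Slingshot actor that teleports between the left and right player positions and can be hidden or shown.
; BeginPlay caches the "pSpot"-tagged actors' locations at the default height, told apart by object name, and moves the slingshot left.
; GoFor switches between the cached spots, while Hide lowers the actor and Show restores its default height.
; The construction script attaches both cable ends to the Holder component.
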(event `GoFor`
  (params (Left :type Boolean))
  ;[1 1 1] Teleporting slingshot for left or right position
  (cast `/Game/Blueprints/SlingshotGameMode` (`GameplayStatics.GetGameMode`))
  (if Left
    (`self.K2_SetActorLocation` (`KismetArrayLibrary.Array_Get` (`self.pPositions`)))
    (else
      (`self.K2_SetActorLocation` (`KismetArrayLibrary.Array_Get` (`self.pPositions`) 1)))))

(event `Hide`
  ;[1 1 1] Hiding slingshot
  (`self.K2_SetActorLocation` (`KismetMathLibrary.MakeVector` (.x (`self.K2_GetActorLocation`)) (.y (`self.K2_GetActorLocation`)) (- (.z (`self.K2_GetActorLocation`)) 50.0))))

(event `Show`
  ;[1 1 1] Showing slingshot
  (`self.K2_SetActorLocation` (`KismetMathLibrary.MakeVector` (.x (`self.K2_GetActorLocation`)) (.y (`self.K2_GetActorLocation`)) (`self.Default Height`))))

(event `self.ReceiveBeginPlay`
  (bind _ppositions (`self.pPositions`))
  ;[1 1 1] Saving players positions on an array
  (bind _outactors (`GameplayStatics.GetAllActorsWithTag` "pSpot"))
  (for _array_element _outactors
    (if (`KismetStringLibrary.EqualEqual_StrStr` (`KismetSystemLibrary.GetObjectName` _array_element) "p1Position")
      (bind _returnvalue (`KismetMathLibrary.MakeVector` (.x (`self.K2_GetActorLocation` _array_element)) (.y (`self.K2_GetActorLocation` _array_element)) (`self.Default Height`)))
      (`KismetArrayLibrary.Array_Set` _ppositions 0 _returnvalue)
      (else
        (`KismetArrayLibrary.Array_Set` _ppositions 1 _returnvalue)))
    (`self.GoFor` true)))

(fn `UserConstructionScript`
  (bind _cable1 (`self.Cable1`))
  (bind _cable2 (`self.Cable2`))
  (`CableComponent.SetAttachEndTo` _cable1 self "Holder" "None")
  (`CableComponent.SetAttachEndTo` _cable2 self "Holder" "None")
  (set `CableComponent.bAttachStart` true _cable1)
  (set `CableComponent.bAttachStart` true _cable2)
  (set `CableComponent.bAttachEnd` true _cable1)
  (set `CableComponent.bAttachEnd` true _cable2))