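; Game instance for a networked two-player slingshot can-knockdown game, running pre-match setup, turn flow, scoring and end screen.
; The server spawns can rows from layout arrays around mirrored pivots and tallies knocked cans per side.
; Turns flip camera and slingshot between sides, respawning cans and projectile.
; Holder moves, launch vectors, scores and turn handshakes pass through the player state, often timed by fixed delays.
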(event `Spawn Cans`
  (params (Turn :type Integer) (AltCanSpawn :type Boolean))
  ;[1 1 1] Spawning actors, removing actors and event bindings
  ;;[1 1 1] Spawning Cans
  (if (`KismetSystemLibrary.IsServer`)
    (if (== Turn 0)
      (`self.Spawn Cans For Player` (`self.CanPositionsP1`) (select `bool` AltCanSpawn :`false` (`self.P1CanCenterPosR`) :`true` (`self.P2CanCenterPosR`)) false Turn)
      (`self.Spawn Cans For Player` (`self.CanPositionsP2`) (select `bool` AltCanSpawn :`false` (`self.P2CanCenterPosR`) :`true` (`self.P1CanCenterPosR`)) true Turn)
      (else
        (`self.Spawn Cans For Player` (`self.CanPositionsP1`) (select `bool` AltCanSpawn :`false` (`self.P1CanCenterPosL`) :`true` (`self.P2CanCenterPosL`)) false Turn true)
        (`self.Spawn Cans For Player` (`self.CanPositionsP2`) (select `bool` AltCanSpawn :`false` (`self.P2CanCenterPosL`) :`true` (`self.P1CanCenterPosL`)) true Turn true)))))

(event `Pre-Match`
  (params (Difficulty :type "/Game/Misc/Enum_Difficulty Enum") (`Cans Per Row` :type Integer) (`Can Scale Bias` :type "Vector Structure") (`Can Size` :type "Vector2D Structure") (`Can Positions P1` :type "Array of /Game/Misc/Enum_CanValues Enum") (`Can Positions P2` :type "Array of /Game/Misc/Enum_CanValues Enum") (`Round Time` :type "Float (double-precision)") (`P1 Color` :type "LinearColor Structure") (`P2 Color` :type "LinearColor Structure") (NOfRounds :type Integer) (CoopPoints :type Integer) (NoCoopPoints :type Integer))
  (bind _slingshot (`self.Slingshot`))
  ;[0 1 0] Pre-Match
  (`self.Set parameters` Difficulty `Cans Per Row` `Can Scale Bias` `Can Size` `Can Positions P1` `Can Positions P2` `Round Time` `P1 Color` `P2 Color` NOfRounds CoopPoints NoCoopPoints)
  (`|ExecutionSequence`
    (:`then_0`
      ;;[1 1 1] Getting Slingshot and Camera References
      (`/Engine/EditorBlueprintResources/StandardMacros.IsValid` (`self.Slingshot`)
        (:`Is Not Valid`
          (bind _returnvalue (`|SpawnActorFromClass` "/Game/Blueprints/Networking/NetworkedSlingshot.NetworkedSlingshot_C" (`KismetMathLibrary.MakeTransform` (0.0 0.0 0.0) (struct :`Yaw` 180.0)) "Undefined" "OverrideRootScale"))
          (set `self.Slingshot` _returnvalue)
          (bind _asslingshot_controller_network (cast `/Game/Blueprints/Networking/SlingshotController_Network` (`GameplayStatics.GetPlayerController` 0)))
          (`/Game/Blueprints/Networking/SlingshotController_Network.Set Slingshot` _asslingshot_controller_network (`self.Slingshot`))
          (bind _returnvalue_2 (`|CreateWidget` "/Game/Huds/W_ScoreHolder.W_ScoreHolder_C"))
          (`UserWidget.AddToViewport` _returnvalue_2 0)
          (set `self.W_ScoreHolder` _returnvalue_2))))
    (:`then_1`
      (bind _outactors (`GameplayStatics.GetAllActorsOfClass` "/Game/Blueprints/Networking/NetworkedCamera.NetworkedCamera_C"))
      (bind _output_get (set `self.MainCamera` (`KismetArrayLibrary.Array_Get` _outactors)))
      (`PlayerController.SetViewTargetWithBlend` (`GameplayStatics.GetPlayerController` 0) _output_get 0.0 "VTBlend_Linear" 0.0 false))
    (:`then_2`
      ;;[1 1 1] Event binds
      (add `/Game/Blueprints/Networking/NetworkedCamera.StartFinished` (`self.MainCamera`) (delegate `StartFinishedDelegate`)))
    (:`then_3`
      ;;[1 1 1] Setting Cans pivot positions
      (bind _outactors_2 (`GameplayStatics.GetAllActorsWithTag` "CanPos"))
      (for _array_element _outactors_2
        (if (`KismetStringLibrary.EqualEqual_StrStr` (`KismetSystemLibrary.GetObjectName` _array_element) "p1CansPos")
          (bind _returnvalue_3 (`Actor.K2_GetActorLocation` _array_element))
          (bind _output_get_2 (set `self.P1CanCenterPosL` _returnvalue_3))
          (set `self.P2CanCenterPosR` (* _output_get_2 (-1.0 1.0 1.0)))
          (else
            (bind _output_get_3 (set `self.P2CanCenterPosL` _returnvalue_3))
            (set `self.P1CanCenterPosR` (* _output_get_3 (-1.0 1.0 1.0)))))))
    (:`then_4`
      ;;[1 1 1] Camera transitions, slingshot's start pose, spawning first cans and ending preparation (pre-match)
      (`|ExecutionSequence`
        (:`then_0`
          (`/Game/Blueprints/Networking/NetworkedCamera.Start To Left` (`self.MainCamera`)))
        (:`then_1`
          (`Actor.SetActorHiddenInGame` _slingshot true)
          (`/Game/Blueprints/Networking/NetworkedSlingshot.GoFor` _slingshot true)
          (`KismetSystemLibrary.Delay` 0.2)
          (`Actor.SetActorHiddenInGame` _slingshot false))
        (:`then_2`
          ;;;[1 1 1] Waiting for player states
          (`KismetSystemLibrary.Delay` 1.0)
          (`self.Send End Pre-match` (`self.Player Data`)))
        (:`then_3`
          (`self.Spawn Cans` (`self.Turn`)))))))

(event `Place ball`
  ;[1 1 1] Spawning actors, removing actors and event bindings
  ;;[1 1 1] Spawns the projectile and bind it's launch to end the turn
  (bind _returnvalue (`|SpawnActorFromClass` "/Game/Blueprints/Networking/NetworkedSlingshot_Projectile.NetworkedSlingshot_Projectile_C" (`KismetMathLibrary.MakeTransform` (0.0 0.0 0.0) (struct)) "Undefined" "OverrideRootScale" null (`self.Difficulty`)))
  (add `/Game/Blueprints/Networking/NetworkedSlingshot_Projectile.Ball Launched` _returnvalue (delegate `Ball launched delegate`))
  (set `self.SpawnedProjectile` _returnvalue))

(event `StartFinishedDelegate`
  ;[0 1 0] Pre-Match
  ;;[1 1 1] Event binds
  (`self.Camera Start Finished`))

(event `Ball launched delegate`
  (params (LeftIntent :type Boolean))
  ;[1 1 1] Spawning actors, removing actors and event bindings
  ;;[1 1 1] Spawns the projectile and bind it's launch to end the turn
  ;;;[1 0 0] End turn on ball launch
  (`self.Send End-Turn` LeftIntent))

(event `Camera Start Finished`
  ;[1 1 1] Spawning actors, removing actors and event bindings
  ;;[1 1 1] Placing ball at the end of camera transition
)

(event `Remove Cans`
  (params (Turn :type Integer))
  (bind _cansleft1 (`self.CansLeft1`))
  (bind _cansleft2 (`self.CansLeft2`))
  (bind _cansright1 (`self.CansRight1`))
  (bind _cansright2 (`self.CansRight2`))
  ;[1 1 1] Spawning actors, removing actors and event bindings
  ;;[1 1 1] Removing Cans
  (`KismetSystemLibrary.Delay` 1.5)
  (switch `int` (mod Turn 2)
    (:`0`
      (for _array_element _cansright1
        (`Actor.K2_DestroyActor` _array_element))
      (`KismetArrayLibrary.Array_Clear` _cansright1)
      (for _array_element_2 _cansright2
        (`Actor.K2_DestroyActor` _array_element_2))
      (`KismetArrayLibrary.Array_Clear` _cansright2))
    (:`1`
      (for _array_element_3 _cansleft1
        (`Actor.K2_DestroyActor` _array_element_3))
      (`KismetArrayLibrary.Array_Clear` _cansleft1)
      (for _array_element_4 _cansleft2
        (`Actor.K2_DestroyActor` _array_element_4))
      (`KismetArrayLibrary.Array_Clear` _cansleft2))))

(event `Receive Launch information from server`
  (params (`Launch Vector` :type "Vector Structure"))
  ;[1 1 1] Communication with Server
  ;;[1 1 1] Receive Launch vector from other client
  (bind _asnetworked_slingshot_projectile (cast `/Game/Blueprints/Networking/NetworkedSlingshot_Projectile` (`KismetArrayLibrary.Array_Get` (`Actor.GetAttachedActors` (`self.Slingshot`)))))
  (`/Game/Blueprints/Networking/NetworkedSlingshot_Projectile.LaunchMe` _asnetworked_slingshot_projectile `Launch Vector` (`KismetMathLibrary.VSize` `Launch Vector`) false false)
  ;;;[1 0 0] Observation turn ended
  (`self.Send End-Turn` false true))

(event `Round Start`
  (params (Turn :type Integer) (AltCanSpawn :type Boolean))
  (bind _spawnedprojectile (`self.SpawnedProjectile`))
  (bind _slingshot (`self.Slingshot`))
  ;[0 1 0] Round has started
  (set `self.usingAltCanSpawn` AltCanSpawn)
  (`self.TurnStartDispatcher`)
  (bind _output_get (set `self.Turn` Turn))
  (`|ExecutionSequence`
    (:`then_0`
      ;;[1 1 1] Slingshot's Position (except for 1st round)
      (if (!= _output_get 1)
        (`Actor.SetActorHiddenInGame` _slingshot true)
        (`/Game/Blueprints/Networking/NetworkedSlingshot.GoFor` _slingshot (`KismetMathLibrary.Conv_IntToBool` (mod (`self.Turn`) 2)))
        (`KismetSystemLibrary.Delay` 0.2)
        (`Actor.SetActorHiddenInGame` _slingshot false)))
    (:`then_1`
      ;;[1 1 1] Setting Slingshot's color based on turn
      (`MeshComponent.SetVectorParameterValueOnMaterials` (`/Game/Blueprints/Networking/NetworkedSlingshot.Slingshot` (`self.Slingshot`)) "PlayerColor" (`KismetMathLibrary.Conv_LinearColorToVector` (select `int` (mod (- (`self.Turn`) 1) 2) :`0` (`self.P1 Color`) :`1` (`self.P2 Color`))))
      (`MeshComponent.SetVectorParameterValueOnMaterials` (`/Game/Blueprints/Networking/NetworkedSlingshot.Holder` (`self.Slingshot`)) "PlayerColor" (`KismetMathLibrary.Conv_LinearColorToVector` (select `int` (mod (- (`self.Turn`) 1) 2) :`0` (`self.P1 Color`) :`1` (`self.P2 Color`)))))
    (:`then_2`
      ;;[1 1 1] Removing previously launched projectile
      (`/Engine/EditorBlueprintResources/StandardMacros.IsValid` _spawnedprojectile
        (:`Is Valid`
          (`Actor.K2_DestroyActor` _spawnedprojectile))))
    (:`then_3`
      (`self.Place ball`))
    (:`then_4`
      ;;[1 1 1] Resetting Launched projectile's control variable
      (bind _asslingshot_controller_network (cast `/Game/Blueprints/Networking/SlingshotController_Network` (`GameplayStatics.GetPlayerController` 0)))
      (set `/Game/Blueprints/Networking/SlingshotController_Network.LaunchedProjectile` false _asslingshot_controller_network))))

(event `Send End Pre-match`
  (params (`Player Data` :type "PlayerData Structure"))
  ;[1 1 1] Communication with Server
  ;;[1 0 0] Send End Pre-match
  (bind _player_state (`self.Get Player State`)
    (:`then`
      (`/Game/Blueprints/Networking/SLingshotPlayerState_Networking.Pre-Match-Ended` _player_state (`KismetSystemLibrary.IsServer`) `Player Data`))))

(event `Receive Slingshots Holder Position`
  (params (`Relative Position` :type "Vector Structure"))
  ;[1 1 1] Communication with Server
  ;;[1 1 1] Receive Slingshots Holder Position from server
  (`SceneComponent.K2_SetRelativeLocation` (`/Game/Blueprints/Networking/NetworkedSlingshot.Holder` (`self.Slingshot`)) `Relative Position` false false))

(event `Update Slingshots Holder Position`
  (params (`Relative position` :type "Vector Structure"))
  ;[1 1 1] Communication with Server
  ;;[1 1 1] Send Slingshots Holder Position to Server on touch movement
  (bind _player_state (`self.Get Player State`)
    (:`then`
      (`/Game/Blueprints/Networking/SLingshotPlayerState_Networking.Send Holder Position to Server` _player_state (`KismetSystemLibrary.IsServer`) `Relative position`))))

(event `Send Launch Information`
  (params (`Launch Vector` :type "Vector Structure"))
  ;[1 1 1] Communication with Server
  ;;[1 1 1] Send Launch Information to server on ball release
  (bind _player_state (`self.Get Player State`)
    (:`then`
      (`/Game/Blueprints/Networking/SLingshotPlayerState_Networking.Send Launch Vector to Server` _player_state `Launch Vector` (`KismetSystemLibrary.IsServer`)))))

(event `Receive players score`
  (params (`P1 Score` :type Integer) (`P2 Score` :type Integer))
  (bind _w_scoreholder (`self.W_ScoreHolder`))
  (bind _returnvalue (`KismetMathLibrary.Conv_IntToDouble` (* (+ (`self.CoopPoints`) (`self.NoCoopPoints`)) (`self.NOfRounds`))))
  ;[1 1 1] Communication with Server
  ;;[1 1 1] Receiving players score from server
  (set `self.P1 Total Score` `P1 Score`)
  (set `self.P2 Total Score` `P2 Score`)
  ;;;[1 0 0] End turn as I've received Scores
  (`self.Send End-turn event has ended`)
  (`/Game/Huds/W_ScoreHolder.Set Percent` _w_scoreholder (/ (`KismetMathLibrary.Conv_IntToDouble` (`self.P1 Total Score`)) _returnvalue) 1)
  (`/Game/Huds/W_ScoreHolder.Set Percent` _w_scoreholder (/ (`KismetMathLibrary.Conv_IntToDouble` (`self.P2 Total Score`)) _returnvalue) 2))

(event `Send End-Turn`
  (params (LeftIntent :type Boolean) (IgnoreIntent :type Boolean))
  ;[1 1 1] Communication with Server
  ;;[1 0 0] Sending End of turn to server
  (`KismetSystemLibrary.Delay` (`self.Round Time`))
  (bind _player_state (`self.Get Player State`)
    (:`then`
      (`/Game/Blueprints/Networking/SLingshotPlayerState_Networking.Send End Turn` _player_state (`KismetSystemLibrary.IsServer`) IgnoreIntent LeftIntent))))

(event `ResetScore`
  (bind _w_scoreholder (`self.W_ScoreHolder`))
  ;[1 1 1] Communication with Server
  ;;[1 1 1] Reset Score
  (`KismetSystemLibrary.Delay` 1.0)
  (`ProgressBar.SetPercent` (`/Game/Huds/W_ScoreHolder.PB_Score_P1` _w_scoreholder) 0.0)
  (`ProgressBar.SetPercent` (`/Game/Huds/W_ScoreHolder.PB_Score_P2` _w_scoreholder) 0.0))

(event `Send End-turn event has ended`
  ;[1 1 1] Communication with Server
  ;;[1 0 0] Sending End-turn event has ended to server
  (`KismetSystemLibrary.Delay` 1.0)
  (bind _player_state (`self.Get Player State`)
    (:`then`
      (`/Game/Blueprints/Networking/SLingshotPlayerState_Networking.Send End-Turn has ended` _player_state (`KismetSystemLibrary.IsServer`)))))

(event `End-Turn`
  (params (Turn :type Integer))
  ;[0 1 0] Start of Ending turn event
  (`self.TurnEndDispatcher`)
  (bind _output_get (set `self.Turn` Turn))
  (`|ExecutionSequence`
    (:`then_0`
      ;;[1 1 1] Change Player location (Camera)
      (`/Game/Blueprints/Networking/NetworkedCamera.Toggle Location` (`self.MainCamera`) (`KismetMathLibrary.Conv_IntToBool` (mod (`self.Turn`) 2))))
    (:`then_1`
      ;;[1 1 1] Spawning Cans
      (`self.Spawn Cans` (mod (+ (`self.Turn`) 1) 2) (`self.usingAltCanSpawn`)))
    (:`then_2`
      (`self.Calculating Score`))
    (:`then_3`
      (`self.Remove Cans` _output_get))))

(event `Send Score to server`
  (params (ServerLaunch :type Boolean))
  ;[1 1 1] Communication with Server
  ;;[1 0 0] Sending Score to Server
  (bind _player_state (`self.Get Player State`)
    (:`then`
      (`/Game/Blueprints/Networking/SLingshotPlayerState_Networking.Send Score to Server` _player_state (`self.p1ScoreInRound`) (`self.p2ScoreInRound`) ServerLaunch))))

(event `Calculating Score`
  ;[1 1 1] Calculating round score
  (set `self.p1ScoreInRound` 0)
  (set `self.p2ScoreInRound` 0)
  (if (`KismetSystemLibrary.IsServer`)
    (`|ExecutionSequence`
      (:`then_0`
        ;;[1 1 1] Server Score
        (for _array_element (`self.CansLeft1`)
          (if (`/Game/Blueprints/Networking/NetworkedSlingshot_Can.Get knockedout` _array_element)
            (switch `/Game/Misc/Enum_CanValues` (`/Game/Blueprints/Networking/NetworkedSlingshot_Can.CanValue` _array_element)
              (:`NewEnumerator0`
                (`/Engine/EditorBlueprintResources/StandardMacros.IncrementInt` (`self.p1ScoreInRound`)))
              (:`NewEnumerator2`
                (`/Engine/EditorBlueprintResources/StandardMacros.IncrementInt` (`self.p2ScoreInRound`))))))
        (for _array_element_2 (`self.CansLeft2`)
          (if (`/Game/Blueprints/Networking/NetworkedSlingshot_Can.Get knockedout` _array_element_2)
            (switch `/Game/Misc/Enum_CanValues` (`/Game/Blueprints/Networking/NetworkedSlingshot_Can.CanValue` _array_element_2)
              (:`NewEnumerator0`
                (`/Engine/EditorBlueprintResources/StandardMacros.IncrementInt` (`self.p1ScoreInRound`)))
              (:`NewEnumerator2`
                (`/Engine/EditorBlueprintResources/StandardMacros.IncrementInt` (`self.p2ScoreInRound`))))))
        ;;;[1 0 0] Sending Score to server
        (`self.Send Score to server` true))
      (:`then_1`
        (set `self.p1ScoreInRound` 0)
        (set `self.p2ScoreInRound` 0)
        ;;[1 1 1] Client score
        (for _array_element_3 (`self.CansRight1`)
          (if (`/Game/Blueprints/Networking/NetworkedSlingshot_Can.Get knockedout` _array_element_3)
            (switch `/Game/Misc/Enum_CanValues` (`/Game/Blueprints/Networking/NetworkedSlingshot_Can.CanValue` _array_element_3)
              (:`NewEnumerator0`
                (`/Engine/EditorBlueprintResources/StandardMacros.IncrementInt` (`self.p2ScoreInRound`)))
              (:`NewEnumerator2`
                (`/Engine/EditorBlueprintResources/StandardMacros.IncrementInt` (`self.p1ScoreInRound`))))))
        (for _array_element_4 (`self.CansRight2`)
          (if (`/Game/Blueprints/Networking/NetworkedSlingshot_Can.Get knockedout` _array_element_4)
            (switch `/Game/Misc/Enum_CanValues` (`/Game/Blueprints/Networking/NetworkedSlingshot_Can.CanValue` _array_element_4)
              (:`NewEnumerator0`
                (`/Engine/EditorBlueprintResources/StandardMacros.IncrementInt` (`self.p2ScoreInRound`)))
              (:`NewEnumerator2`
                (`/Engine/EditorBlueprintResources/StandardMacros.IncrementInt` (`self.p1ScoreInRound`))))))
        ;;;[1 0 0] Sending Score to server
        (`self.Send Score to server` false)))))

(event `End Game`
  ;[0 1 0] Game end
  (bind _returnvalue (`|CreateWidget` "/Game/Huds/W_EndGame.W_EndGame_C"))
  (`UserWidget.AddToViewport` _returnvalue 0))

(event `TCP`
  ;[1 0 0.7206] Launch TCP function to connect to the server to find the other player
  (bind _returnvalue (`|SpawnActorFromClass` "/Script/Estilingue.TCPActor" (`KismetMathLibrary.MakeTransform` (0.0 0.0 0.0)) "Undefined" "OverrideRootScale"))
  (bind _output_get (set `self.TCPActor` _returnvalue))
  (`TCPActor.Launch` _output_get))

(event `self.HandleNetworkError`
  (params (FailureType :type "ENetworkFailure Enum" :default "NetDriverAlreadyExists") (bIsServer :type Boolean))
  ;[1 0 1] Handling network errors
  (switch `ENetworkFailure` FailureType
    (:`ConnectionLost`
      _)
    (:`ConnectionTimeout`
      _)
    (:`FailureReceived`
      _)
    (:`PendingConnectionFailure`
      _))
  (if bIsServer
    _
    (else
      _))
  (bind _returnvalue (`|CreateWidget` "/Game/Huds/W_ErrorMessages.W_ErrorMessages_C"))
  (`UserWidget.AddToViewport` _returnvalue 0)
  (`TextBlock.SetText` (`/Game/Huds/W_ErrorMessages.ErrorMessage` _returnvalue) (select `ENetworkFailure` FailureType :`ConnectionLost` "Conexão perdida" :`ConnectionTimeout` "Conexão timeout" :`FailureReceived` "Falha de conexão" :`PendingConnectionFailure` "Prestes a perder conexão" :!type "Text")))

(event `Send Player Data to server`
  ;[1 0 0] Sending Player data to server as requested on match start
  (`KismetSystemLibrary.Delay` 0.5)
  (bind _player_state (`self.Get Player State`)
    (:`then`
      (`/Game/Blueprints/Networking/SLingshotPlayerState_Networking.Send Player Data to server` _player_state (`self.Player Data`) (`KismetSystemLibrary.IsServer`) (`self.SelectedColor`) (`self.usingResearchMode`)))))

(event `Send Replay intent`
  ;[1 0 0] Send replay intent to server on Play Again action
  (bind _player_state (`self.Get Player State`)
    (:`then`
      (`/Game/Blueprints/Networking/SLingshotPlayerState_Networking.Send replay intent to server` _player_state (`KismetSystemLibrary.IsServer`)))))

(fn `Calculate Can Transform`
  (params (ArrayIndex :type Integer) (`Can Center Pos` :type "Vector Structure") (CanCenterIndex :type Integer) (CurrentRow :type Integer) (IsRight :type Boolean))
  (returns (X :type "Float (double-precision)") (Y :type "Float (double-precision)") (Z :type "Float (double-precision)") (IndexOnRow :type Integer))
  (bind _y (.y `Can Center Pos`))
  (bind _x (`KismetMathLibrary.BreakVector2D` (`self.CanSize`)))
  (bind _returnvalue (mod ArrayIndex (`self.CansPerRow`)))
  (bind _returnvalue_2 (+ (.z `Can Center Pos`) (* CurrentRow (`.Y` (`KismetMathLibrary.BreakVector2D` (`self.CanSize`))))))
  (bind _returnvalue_3 (+ (* (- CanCenterIndex _returnvalue) _x) (.x `Can Center Pos`)))
  ;[1 1 1] Calculating Can Transform
  (if IsRight
    (return (- _returnvalue_3 (* _x (`KismetMathLibrary.Conv_IntToDouble` (- (`self.CansPerRow`) 1)))) _y _returnvalue_2 _returnvalue)
    (else
      (return _returnvalue_3 _y _returnvalue_2 _returnvalue))))

(fn `Set parameters`
  (params (Difficulty :type "/Game/Misc/Enum_Difficulty Enum") (`Cans per row` :type Integer) (`Can Scale Bias` :type "Vector Structure") (`Can Size` :type "Vector2D Structure") (`Can Positions P1` :type "Array of /Game/Misc/Enum_CanValues Enum") (`Can Positions P2` :type "Array of /Game/Misc/Enum_CanValues Enum") (`Round Time` :type "Float (double-precision)") (`P1 Color` :type "LinearColor Structure") (`P2 Color` :type "LinearColor Structure") (NOfRounds :type Integer) (CoopPoints :type Integer) (NoCoopPoints :type Integer))
  (set `self.CansPerRow` `Cans per row`)
  (set `self.Difficulty` Difficulty)
  (set `self.CanScale` `Can Scale Bias`)
  (set `self.CanSize` `Can Size`)
  (set `self.CanPositionsP1` `Can Positions P1`)
  (set `self.CanPositionsP2` `Can Positions P2`)
  (set `self.Round Time` `Round Time`)
  (set `self.P1 Color` `P1 Color`)
  (set `self.P2 Color` `P2 Color`)
  (set `self.NOfRounds` NOfRounds)
  (set `self.CoopPoints` CoopPoints)
  (set `self.NoCoopPoints` NoCoopPoints))

(fn `Spawn Cans for Player`
  (params (PlayerCansPositions :type "Array of /Game/Misc/Enum_CanValues Enum") (`Player Pivot Position` :type "Vector Structure") (IsRight :type Boolean) (Turn :type Integer) (IsASide :type Boolean))
  (locals (CanCenterIndex :type Integer) (CurrentRow :type Integer :default -1) (LocalTurn :type Integer) (NeutralColor :type "LinearColor Structure" :default (struct :`R` 0.735 :`G` 0.735 :`B` 0.735)))
  (bind _returnvalue (mod (`local.LocalTurn`) 2))
  (bind _returnvalue_2 (mod (`self.CansPerRow`) 2))
  ;[1 1 1] Central index calculation
  (set `local.LocalTurn` Turn)
  (if (== _returnvalue_2 0)
    (set `local.CanCenterIndex` _returnvalue_2)
    (else
      (set `local.CanCenterIndex` (+ _returnvalue_2 1))))
  (for (_array_element _array_index) PlayerCansPositions
    (bind (_x _y _z _indexonrow) (`self.Calculate Can Transform` _array_index `Player Pivot Position` (`local.CanCenterIndex`) (`local.CurrentRow`) IsRight))
    ;[1 1 1] Checking to increment row based on array index
    (if (== _indexonrow 0)
      (`/Engine/EditorBlueprintResources/StandardMacros.IncrementInt` (`local.CurrentRow`)
        (:`  `
          _)))
    (switch `/Game/Misc/Enum_CanValues` _array_element
      (:`NewEnumerator0`
        (bind _returnvalue_3 (`KismetMathLibrary.MakeTransform` (`KismetMathLibrary.MakeVector` _x _y _z) (struct) (`self.CanScale`)))
        (bind _returnvalue_4 (`|SpawnActorFromClass` "/Game/Blueprints/Networking/NetworkedSlingshot_Can.NetworkedSlingshot_Can_C" _returnvalue_3 "Undefined" "OverrideRootScale" null _returnvalue _array_index _array_element))
        ;[1 1 1] Coloring Cans
        (`/Game/Blueprints/Networking/NetworkedSlingshot_Can.Change Material` _returnvalue_4 (select `int` (mod (`local.LocalTurn`) 2) :`0` (`self.P2 Color`) :`1` (`self.P1 Color`))))
      (:`NewEnumerator1`
        (bind _returnvalue_5 (`|SpawnActorFromClass` "/Game/Blueprints/Networking/NetworkedSlingshot_Can.NetworkedSlingshot_Can_C" _returnvalue_3 "Undefined" "OverrideRootScale" null _returnvalue _array_index _array_element))
        (`/Game/Blueprints/Networking/NetworkedSlingshot_Can.Change Material` _returnvalue_5 (`local.NeutralColor`)))
      (:`NewEnumerator2`
        (bind _returnvalue_6 (`|SpawnActorFromClass` "/Game/Blueprints/Networking/NetworkedSlingshot_Can.NetworkedSlingshot_Can_C" _returnvalue_3 "Undefined" "OverrideRootScale" null _returnvalue _array_index _array_element))
        (`/Game/Blueprints/Networking/NetworkedSlingshot_Can.Change Material` _returnvalue_6 (select `int` (mod (`local.LocalTurn`) 2) :`0` (`self.P1 Color`) :`1` (`self.P2 Color`)))))
    ;[1 1 1] Filling cans arrays with proper cans
    (if (and (not IsRight) IsASide)
      (bind _returnvalue_7 (select `/Game/Misc/Enum_CanValues` _array_element :`NewEnumerator0` _returnvalue_4 :`NewEnumerator1` _returnvalue_5 :`NewEnumerator2` _returnvalue_6))
      (`KismetArrayLibrary.Array_Add` (`self.CansLeft1`) _returnvalue_7)
      (elif (and IsRight IsASide)
        (`KismetArrayLibrary.Array_Add` (`self.CansLeft2`) _returnvalue_7)
        (elif (and (not IsASide) (not IsRight))
          (`KismetArrayLibrary.Array_Add` (`self.CansRight1`) _returnvalue_7)
          (elif (and IsRight (not IsASide))
            (`KismetArrayLibrary.Array_Add` (`self.CansRight2`) _returnvalue_7)))))))