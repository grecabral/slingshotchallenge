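; Touch controller for a turn-based slingshot game that lets the player drag and fire projectiles and exposes a BotLaunch event for bot shots.
; While a touch begun on the Slingshot moves, a Gate feeds finger traces into clamped Holder positions.
; Release launches attached projectiles along the Holder-to-AimPosition vector, fires the launch dispatcher and resets the Holder.
; CheckBotTurn limits touch to player turns; TrajectoryVisualizer spawning is unconnected.
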(event `Bot Launch`
  (params (Direction :type "Vector Structure"))
  ;[1 1 1] Bot Launch
  (for _array_element (`self.GetAttachedActors` (`self.Slingshot`))
    (bind _asslingshot_projectile (cast `/Game/Blueprints/Slingshot_Projectile` _array_element))
    (`/Game/Blueprints/Slingshot_Projectile.LaunchMe` _asslingshot_projectile Direction (`KismetMathLibrary.VSize` Direction))
    (`self.Launch Dispatcher` (< (.x Direction) 0.0))))

(event `self.ReceiveTick`
  (params (DeltaSeconds :type "Float (single-precision)"))
  ;[1 1 1] On release
)

(event `self.ReceiveBeginPlay`
  ;[1 1 1] Getting Slingshot Reference
  (bind _outactors (`GameplayStatics.GetAllActorsOfClass` "/Game/Blueprints/Slingshot.Slingshot_C"))
  (set `self.Slingshot` (`KismetArrayLibrary.Array_Get` _outactors)))

(event `InputTouch`
  (params (Location :type "Vector Structure") (FingerIndex :type "ETouchIndex Enum"))
  (bind _slingshot (`self.Slingshot`))
  (bind _slingshot_2 (`self.Slingshot`))
  (bind (_hitresult _returnvalue) (`self.GetHitResultUnderFingerForObjects` "Touch1" (`|MakeArray` "ObjectTypeQuery8" :!type "EObjectTypeQuery Enum")))
  (bind (_x _y) (`KismetMathLibrary.BreakVector2D` (`self.ClampBounds`)))
  (bind (_x_2 _y_2) (`KismetMathLibrary.BreakVector2D` (`self.ClampBounds`)))
  (bind _x_3 (`KismetMathLibrary.BreakVector2D` (`self.ClampBounds`)))
  (bind _holder (`/Game/Blueprints/Slingshot.Holder` _slingshot))
  (bind _z (.z (.location (`SceneComponent.GetRelativeTransform` (`/Game/Blueprints/Slingshot.Aim` _slingshot)))))
  (bind _x_4 (.x (- (`SceneComponent.K2_GetComponentLocation` (`/Game/Blueprints/Slingshot.AimPosition` _slingshot_2)) (`SceneComponent.K2_GetComponentLocation` (`/Game/Blueprints/Slingshot.Holder` _slingshot_2)))))
  (bind _z_2 (.z (- (`SceneComponent.K2_GetComponentLocation` (`/Game/Blueprints/Slingshot.AimPosition` _slingshot_2)) (`SceneComponent.K2_GetComponentLocation` (`/Game/Blueprints/Slingshot.Holder` _slingshot_2)))))
  (bind _y_3 (.y (.location (`SceneComponent.GetRelativeTransform` _holder))))
  (bind _returnvalue_2 (`KismetMathLibrary.MakeVector` _x_4 _z_2 _z_2))
  (bind _returnvalue_3 (- (`KismetMathLibrary.Abs` (.x (`.Location` (`GameplayStatics.BreakHitResult` _hitresult)))) (+ (.x (.location (`SceneComponent.GetRelativeTransform` (`/Game/Blueprints/Slingshot.Aim` _slingshot)))) (.x (`self.K2_GetActorLocation` _slingshot)))))
  (bind _returnvalue_4 (* _returnvalue_3 -1.0))
  (bind _returnvalue_5 (+ _z (- (.z (`.Location` (`GameplayStatics.BreakHitResult` _hitresult))) (+ _z (.z (`self.K2_GetActorLocation` _slingshot))))))
  ;[1 1 1] Setting Slingshot's holder position
  (:`Pressed`
    (`self.Check Bot Turn`)
    (if (== (`.HitActor` (`GameplayStatics.BreakHitResult` (`self.GetHitResultUnderFingerForObjects` "Touch1" (`|MakeArray` "ObjectTypeQuery7" :!type "EObjectTypeQuery Enum")))) (`self.Slingshot`))
      (set `self.isPressedOnSlingshot` true)
      (goto _label :!via `Open`)))
  (:`Released`
    (`self.Check Bot Turn`)
    (`|ExecutionSequence`
      (:`then_0`
        ;[1 1 1] On release
        (if (`self.isPressedOnSlingshot`)
          (for _array_element (`self.GetAttachedActors` _slingshot_2)
            (bind _asslingshot_projectile (cast `/Game/Blueprints/Slingshot_Projectile` _array_element))
            (if (not (`self.LaunchedProjectile`))
              (`/Game/Blueprints/Slingshot_Projectile.LaunchMe` _asslingshot_projectile _returnvalue_2 (`KismetMathLibrary.VSize` _returnvalue_2))
              (set `self.LaunchedProjectile` true)
              (`self.Launch Dispatcher` (< _x_4 0.0))))))
      (:`then_1`
        (`SceneComponent.K2_SetRelativeLocation` _holder (`KismetMathLibrary.MakeVector` 0.0 _y_3 _z) false false))
      (:`then_2`
        (set `self.isPressedOnSlingshot` false)
        (goto _label :!via `Close`))))
  (:`Moved`
    (`self.Check Bot Turn`)
    (`/Engine/EditorBlueprintResources/StandardMacros.Gate` true :!label _label
      (:`Exit`
        (if (not (`self.LaunchedProjectile`))
          (set `self.SlingY` _y_3)
          (`|ExecutionSequence`
            (:`then_0`
              ;;[1 1 1] Clamping X and Z
              ;;;[1 1 1] Clamping X
              (if (> (`KismetMathLibrary.Abs` _returnvalue_3) _x_2)
                (if (< _returnvalue_4 0.0)
                  (set `self.SlingX` (* _x_3 -1.0))
                  (else
                    (set `self.SlingX` _x_3)))
                (else
                  (set `self.SlingX` _returnvalue_4))))
            (:`then_1`
              ;;;[1 1 1] Clamping Z
              (if (> (`KismetMathLibrary.Abs` _returnvalue_5) _y_2)
                (if false
                  (set `self.SlingZ` (* _y -1.0))
                  (else
                    (set `self.SlingZ` _y)))
                (else
                  (set `self.SlingZ` _returnvalue_5))))
            (:`then_2`
              (if _returnvalue
                (`SceneComponent.K2_SetRelativeLocation` _holder (`KismetMathLibrary.MakeVector` (`self.SlingX`) (`self.SlingY`) (`self.SlingZ`)) false false)))))))))

(fn `UserConstructionScript`)