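; Game mode for the main menu, managing the flow between menu, player info and match data screens.
; On BeginPlay it shows the main menu widget and spawns an HTTP actor.
; Start stores the multiplayer flag on the networking game instance and opens player info; screens are created on first use, then toggled by visibility.
; Returning from match data resets that flag to false; single player opens the Suburb_SP level.
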(event `self.ReceiveBeginPlay`
  ;[1 1 1] Main menu widget on begin
  (bind _returnvalue (`|CreateWidget` "/Game/Huds/W_MainMenu.W_MainMenu_C"))
  (bind _output_get (set `self.Menu Widget` _returnvalue))
  (`UserWidget.AddToViewport` _output_get 0)
  ;[1 1 1] HTTP Actor
  (`|SpawnActorFromClass` "/Game/Blueprints/Networking/BP_HttpActor.BP_HttpActor_C" (`KismetMathLibrary.MakeTransform` (0.0 0.0 0.0)) "Undefined" "OverrideRootScale"))

(event `Back to main menu`
  (bind _player_info_widget (`self.Player Info Widget`))
  (bind _match_data_widget (`self.Match Data Widget`))
  (bind _menu_widget (`self.Menu Widget`))
  ;[1 1 1] Back to main menu
  (`/Engine/EditorBlueprintResources/StandardMacros.IsValid` _player_info_widget
    (:`Is Valid`
      (`Widget.SetVisibility` _player_info_widget "Hidden")
      (`Widget.SetIsEnabled` _player_info_widget true))
    (:`Is Not Valid`
      _))
  (`/Engine/EditorBlueprintResources/StandardMacros.IsValid` _match_data_widget
    (:`Is Valid`
      (`Widget.SetVisibility` _match_data_widget "Hidden"))
    (:`Is Not Valid`
      _))
  (`/Engine/EditorBlueprintResources/StandardMacros.IsValid` _menu_widget
    (:`Is Valid`
      (`Widget.SetVisibility` _menu_widget "Visible"))))

(event `Start`
  (params (isMP :type Boolean))
  (bind _player_info_widget (`self.Player Info Widget`))
  ;[1 1 1] Show player info widget
  (bind _output_get (set `self.isMp` isMP))
  (bind _asslingshot_game_instance_networking (cast `/Game/Blueprints/SlingshotGameInstance_Networking` (`GameplayStatics.GetGameInstance`)))
  (set `/Game/Blueprints/SlingshotGameInstance_Networking.IsMP` _output_get _asslingshot_game_instance_networking)
  (if (`Widget.IsVisible` (`self.Menu Widget`))
    (`Widget.SetVisibility` (`self.Menu Widget`) "Hidden"))
  (`/Engine/EditorBlueprintResources/StandardMacros.IsValid` _player_info_widget
    (:`Is Valid`
      (`Widget.SetVisibility` _player_info_widget "Visible"))
    (:`Is Not Valid`
      (bind _returnvalue (`|CreateWidget` "/Game/Huds/W_PlayerInfo.W_PlayerInfo_C"))
      (bind _output_get_2 (set `self.Player Info Widget` _returnvalue))
      (`UserWidget.AddToViewport` _output_get_2 0))))

(event `Show Match Data Widget`
  (bind _match_data_widget (`self.Match Data Widget`))
  ;[1 1 1] Show Match Data
  (`Widget.SetVisibility` (`self.Player Info Widget`) "Hidden")
  (`/Engine/EditorBlueprintResources/StandardMacros.IsValid` _match_data_widget
    (:`Is Valid`
      (`Widget.SetVisibility` _match_data_widget "Visible"))
    (:`Is Not Valid`
      (bind _returnvalue (`|CreateWidget` "/Game/Huds/W_MatchData.W_MatchData_C"))
      (bind _output_get (set `self.Match Data Widget` _returnvalue))
      (`UserWidget.AddToViewport` _output_get 0))))

(event `Back to player info menu`
  (bind _match_data_widget (`self.Match Data Widget`))
  ;[1 1 1] Back to player info
  (`/Engine/EditorBlueprintResources/StandardMacros.IsValid` _match_data_widget
    (:`Is Valid`
      (`Widget.SetVisibility` _match_data_widget "Hidden")
      (`self.Start` false))))

(event `Start Single Player`
  ;[1 1 1] Start Single Player
  (`GameplayStatics.OpenLevel` "Suburb_SP"))

(fn `UserConstructionScript`)