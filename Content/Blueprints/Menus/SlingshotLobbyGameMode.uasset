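; Lobby game mode for a two-player match, which shows the match data widget and spawns an HTTP actor on BeginPlay.
; Tick waits until CanStart is set and two players are present, then server-travels to Suburb_MP.
; An IsTraveling flag suppresses the "Player 2 saiu" error widget during travel, so it only appears when a remote player leaves the lobby.
; A separate event returns to the main menu.
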(event `self.ReceiveBeginPlay`
  ;[1 1 1] Only server creates widget
  (set `self.isTraveling` false)
  (bind _returnvalue (`|CreateWidget` "/Game/Huds/W_MatchData.W_MatchData_C"))
  (`UserWidget.AddToViewport` _returnvalue 0)
  ;[1 1 1] HTTP Actor
  (`|SpawnActorFromClass` "/Game/Blueprints/Networking/BP_HttpActor.BP_HttpActor_C" (`KismetMathLibrary.MakeTransform` (0.0 0.0 0.0)) "Undefined" "OverrideRootScale"))

(event `Back to main menu`
  (`GameplayStatics.OpenLevel` "MainMenu"))

(event `self.K2_OnLogout`
  (params (ExitingController :type "Controller Object Reference"))
  ;[1 0 1] Client disconnected
  (if (and (not (`Controller.IsLocalController` ExitingController)) (not (`self.IsTraveling`)))
    (bind _returnvalue (`|CreateWidget` "/Game/Huds/W_ErrorMessages.W_ErrorMessages_C"))
    (`UserWidget.AddToViewport` _returnvalue 0)
    (`TextBlock.SetText` (`/Game/Huds/W_ErrorMessages.ErrorMessage` _returnvalue) "Player 2 saiu")))

(event `self.ReceiveTick`
  (params (DeltaSeconds :type "Float (single-precision)"))
  ;[1 1 1] Checking if we can proceed to launch the game, happens on successfully setting match data from server
  (if (and (`self.canStart`) (== (`KismetArrayLibrary.Array_Length` (`GameStateBase.PlayerArray` (`GameplayStatics.GetGameState`))) 2))
    (set `self.isTraveling` true)
    (`KismetSystemLibrary.ExecuteConsoleCommand` "ServerTravel Suburb_MP")))

(fn `UserConstructionScript`)