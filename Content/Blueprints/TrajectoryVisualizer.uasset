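; TrajectoryVisualizer is a short-lived projectile actor that, by its name, previews the path of a Slingshot shot.
; After a brief delay on BeginPlay it sets its lifespan and snaps to the Holder of the first Slingshot found, keeping world rotation and scale.
; It then sets ProjectileMovement velocity from its Direction variable with fixed per-axis scaling and activates the movement.
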(event `self.ReceiveBeginPlay`
  (bind _projectilemovement (`self.ProjectileMovement`))
  (`KismetSystemLibrary.Delay` 0.2)
  (`self.SetLifeSpan` 3.0)
  (bind _outactors (`GameplayStatics.GetAllActorsOfClass` "/Game/Blueprints/Slingshot.Slingshot_C"))
  (`self.K2_AttachToComponent` (`/Game/Blueprints/Slingshot.Holder` (`KismetArrayLibrary.Array_Get` _outactors)) "None" "SnapToTarget" "KeepWorld" "KeepWorld")
  (set `MovementComponent.Velocity` (* (`self.Direction`) (50.0 90.0 70.0)) _projectilemovement)
  (`ActorComponent.SetActive` _projectilemovement true false))

(fn `UserConstructionScript`)